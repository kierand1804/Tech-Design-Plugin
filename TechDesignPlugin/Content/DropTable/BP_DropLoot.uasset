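; BP_DropLoot is a component that drops a random item from its owning actor and then destroys that owner.
; GiveLoot traces 200 units down from the owner to find the drop point, ignoring the player character.
; RandomizeLoot picks a row uniformly from DT_LootTable, prints its name and stores its item class.
; GiveLoot spawns that class at the trace hit location with a random yaw.
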(event Custom|GiveLoot
  (bind _returnvalue (Components|GetOwner))
  (bind _returnvalue_2 (Transformation|GetActorLocation _returnvalue))
  (bind _outhit (Collision|LineTraceByChannel _returnvalue_2 (- _returnvalue_2 "0.000000,0.000000,200.000000") "TraceTypeQuery1" false (Utilities|Array|MakeArray (Game|GetPlayerCharacter 0)) "None"))
  (CallFunction|RandomizeLoot)
  (Game|SpawnActorfromClass (Variables|Default|GetItem) (Math|Transform|MakeTransform (.Location (Collision|BreakHitResult _outhit)) (Math|Rotator|MakeRotator 0.0 0.0 (Math|Random|RandomFloatinRange 0.0 3.6e+02))) "Undefined" "MultiplyWithRoot" 0 0)
  (Actor|DestroyActor (Components|GetOwner)))

(event EventBeginPlay)

(event EventTick
  (params (DeltaSeconds :type Float%20%28single-precision%29)))

(fn RandomizeLoot
  (bind _outrownames (DataTable|GetDataTableRowNames "/TechDesignPlugin/DropTable/Editable/DT_LootTable.DT_LootTable"))
  (bind _returnvalue (Utilities|GetDataTableRow "/TechDesignPlugin/DropTable/Editable/DT_LootTable.DT_LootTable" (.OutItem (Utilities|Array|Random _outrownames)))
    (:then
      (Development|PrintString (.Name (Utilities|Struct|BreakStruct_Loot _returnvalue)))
      (Variables|Default|SetItem (.Item (Utilities|Struct|BreakStruct_Loot _returnvalue))))))